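; BP_Workshop is a workshop structure in an RTS game that shows a message through its widget component.
; On BeginPlay it runs parent logic and registers itself with the widget as the message actor.
; The widget message appears when the workshop is selected or when an RTS base character enters its sphere.
; The end-overlap handler only casts the actor, so leaving the sphere triggers nothing here.
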(event `self.ReceiveBeginPlay`
  (`parent.ReceiveBeginPlay`)
  (message `RTSUIInterfaces.SetActor` (`WidgetComponent.GetUserWidgetObject` (`self.Widget`)) self))

(event `self.Sphere.OnComponentBeginOverlap`
  (params (OverlappedComponent :type "PrimitiveComponent Object Reference") (OtherActor :type "Actor Object Reference") (OtherComp :type "PrimitiveComponent Object Reference") (OtherBodyIndex :type Integer) (bFromSweep :type Boolean) (SweepResult :type "HitResult Structure (by ref)"))
  (cast `/Game/Core/BP_RTSBaseCharacters` OtherActor)
  (message `RTSUIInterfaces.OnShow` (`WidgetComponent.GetUserWidgetObject` (`self.Widget`))))

(event `self.Sphere.OnComponentEndOverlap`
  (params (OverlappedComponent :type "PrimitiveComponent Object Reference") (OtherActor :type "Actor Object Reference") (OtherComp :type "PrimitiveComponent Object Reference") (OtherBodyIndex :type Integer))
  (cast `/Game/Core/BP_RTSBaseCharacters` OtherActor))

(event `self.OnSelect`
  (`parent.OnSelect`)
  (message `RTSUIInterfaces.OnShow` (`WidgetComponent.GetUserWidgetObject` (`self.Widget`))))

(fn `UserConstructionScript`
  (`parent.UserConstructionScript`))