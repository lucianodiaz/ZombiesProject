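; Base Blueprint for RTS characters, with a gender-based appearance and player-issued target locations.
; SetCharacterInfo stores the character info and picks the male or female mannequin mesh and animation Blueprint from its Genre.
; OnSelect defers to the parent class, while OnAction also copies the RTS player controller's TargetLocation into the character's AI blackboard.
; From BeginPlay, a looping timer makes every instance steadily damage itself.
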(event `self.ReceiveBeginPlay`
  (`parent.ReceiveBeginPlay`)
  (`KismetSystemLibrary.K2_SetTimerDelegate` (delegate `KillEverione`) 1.8 true))

(event `KillEverione`
  (`GameplayStatics.ApplyDamage` self 2.0))

(event `SetCharacterInfo`
  (params (CharaterInfo :type "CharacterInfo Structure"))
  (set `self.Charater Info` CharaterInfo)
  (switch `string` (`KismetTextLibrary.Conv_TextToString` (`.Genre` (break `CharacterInfo` (`self.Charater Info`))))
    (:`M`
      (`SkinnedMeshComponent.SetSkinnedAssetAndUpdate` (`self.Mesh`) "/Game/ODSMannequin/Mannequin/Character/Mesh/SK_Mannequin.SK_Mannequin" true)
      (`SkeletalMeshComponent.SetAnimInstanceClass` (`self.Mesh`) "/Game/ODSMannequin/Mannequin/Animations/ThirdPerson_AnimBP.ThirdPerson_AnimBP_C"))
    (:`F`
      (`SkinnedMeshComponent.SetSkinnedAssetAndUpdate` (`self.Mesh`) "/Game/ODSMannequin/FemaleMannequin/Character/Mesh/SK_FemaleMannequin.SK_FemaleMannequin" true)
      (`SkeletalMeshComponent.SetAnimInstanceClass` (`self.Mesh`) "/Game/ODSMannequin/FemaleMannequin/Animations/FemaleMannequin_AnimBP.FemaleMannequin_AnimBP_C"))))

(event `self.OnSelect`
  (`parent.OnSelect`))

(event `self.OnAction`
  (`parent.OnAction`)
  (bind _asrtsplayer_controller (cast `RTSPlayerController` (`GameplayStatics.GetPlayerController` 0)))
  (`/Engine/EditorBlueprintResources/StandardMacros.IsValid` (`AIBlueprintHelperLibrary.GetBlackboard` self)
    (:`Is Valid`
      (`BlackboardComponent.SetValueAsVector` (`AIBlueprintHelperLibrary.GetBlackboard` self) "TargetLocation" (`RTSPlayerController.TargetLocation` _asrtsplayer_controller)))))

(fn `UserConstructionScript`)