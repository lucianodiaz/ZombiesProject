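; BP_ObjectInteractable is an interactable object that highlights its Cube in magenta while selected.
; On BeginPlay it creates a dynamic material instance on the Cube and caches the original Color parameter.
; OnSelect and OnDeselect extend the parent's events, setting that parameter to the highlight color and restoring the cached color respectively.
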(event `self.ReceiveBeginPlay`
  (bind _returnvalue (`PrimitiveComponent.CreateDynamicMaterialInstance` (`self.Cube`) 0 null "None"))
  (bind _output_get (set `self.MaterialInstance` _returnvalue))
  (bind _returnvalue_2 (`MaterialInstanceDynamic.K2_GetVectorParameterValue` _output_get "Color"))
  (set `self.BaseColor` _returnvalue_2))

(event `self.OnSelect`
  (`parent.OnSelect`)
  (`MaterialInstanceDynamic.SetVectorParameterValue` (`self.MaterialInstance`) "Color" (struct :`R` 1.0 :`B` 0.927672 :`A` 1.0)))

(event `self.OnDeselect`
  (`parent.OnDeselect`)
  (`MaterialInstanceDynamic.SetVectorParameterValue` (`self.MaterialInstance`) "Color" (`self.BaseColor`)))

(fn `UserConstructionScript`)