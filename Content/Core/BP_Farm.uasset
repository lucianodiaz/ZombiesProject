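; BP_Farm is a farm actor that yields a set type and amount of resource to the game mode.
; A looping five-second timer tells its widget component, which holds a reference to the farm, to show a pop-up.
; OnEndAction restarts that timer and sends the resource to the game mode through a message call.
; ReturnType exposes the type and count, while the selection events are empty stubs.
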(event `self.ReceiveBeginPlay`
  (`parent.ReceiveBeginPlay`)
  (message `RTSUIInterfaces.SetActor` (`WidgetComponent.GetUserWidgetObject` (`self.Widget`)) self)
  (message `RTSUIInterfaces.OnHide` (`WidgetComponent.GetUserWidgetObject` (`self.Widget`)))
  (`KismetSystemLibrary.K2_SetTimer` null "ShowPopUp" 5.0 true))

(event `ShowPopUp`
  (message `RTSUIInterfaces.OnShow` (`WidgetComponent.GetUserWidgetObject` (`self.Widget`))))

(event `/Game/Blueprints/Interfaces/BPI_BuildInterface.OnEndAction`
  (`KismetSystemLibrary.K2_SetTimer` null "ShowPopUp" 5.0 true)
  (message `/Game/Blueprints/Interfaces/BPI_GMInterface.AddResources` (`GameplayStatics.GetGameMode`) (`self.ResourceType`) (`self.Count`)))

(event `self.OnSelect`)

(event `self.OnDeselect`)

(fn `ReturnType`
  (returns (NewParam :type "/Game/Core/ResourcesType Enum") (count :type Integer))
  (return (`self.ResourceType`) (`self.Count`)))

(fn `UserConstructionScript`
  (`parent.UserConstructionScript`))