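; City builder game mode that assigns identities to the base RTS characters and keeps the resource counts.
; On BeginPlay it loads character rows from a data table and gives each a random thumbnail matching its gender.
; Each placed character gets an unused random entry, found by recursive retry with no exhaustion guard.
; The character count is added to the People resource through AddResources, and GetResources exposes the totals.
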(event `self.ReceiveBeginPlay`
  (`self.SetCharacterInfo`)
  (bind _outactors (`GameplayStatics.GetAllActorsOfClass` "/Game/Core/BP_RTSBaseCharacters.BP_RTSBaseCharacters_C"))
  (bind _output_get (set `self.BasePlayers` _outactors))
  (for _array_element _output_get
    (bind _newparam (`self.GetCharacterInfo`))
    (`/Game/Core/BP_RTSBaseCharacters.SetCharacterInfo` _array_element _newparam))
  (`self.AddResources` "People" (`KismetArrayLibrary.Array_Length` (`self.BasePlayers`))))

(event `self.AddResources`
  (params (ResourceType :type "EResourceType Enum" :default "Food") (Ammout :type Integer))
  ;[1 1 1] Add Resources
  (for (_array_element _array_index) (`self.Resources`)
    (bind (_thumbnail _resourcename _resourcetype _count) (break `ResourceInfo` _array_element))
    (if (`|EnumEquality` ResourceType _resourcetype)
      (bind _structout (setmembers `ResourceInfo` :`StructRef` _array_element :`Count` (+ _count Ammout)))
      (`KismetArrayLibrary.Array_Set` (`self.Resources`) _array_index _structout))))

(fn `GetCharacterInfo`
  (returns (NewParam :type "/Game/Blueprints/Data/CharacterInfo Structure"))
  (locals (RandomInfo :type "/Game/Blueprints/Data/CharacterInfo Structure") (Index :type Integer))
  (bind (_outitem _outindex) (`KismetArrayLibrary.Array_Random` (`self.AvatarsInfo`)))
  (set `local.RandomInfo` _outitem)
  (set `local.Index` _outindex)
  (if (`.inUse_16_5E2B92034D3108A8E75F2693D6FB6F46` (break `/Game/Blueprints/Data/CharacterInfo` (`local.RandomInfo`)))
    (bind _newparam (`self.GetCharacterInfo`))
    (return _newparam)
    (else
      (bind _structout (setmembers `/Game/Blueprints/Data/CharacterInfo` :`StructRef` (`local.RandomInfo`) :`inUse` true))
      (`KismetArrayLibrary.Array_Set` (`self.AvatarsInfo`) (`local.Index`) _structout)
      (return _structout))))

(fn `GetResources`
  (returns (NewParam :type "Array of ResourceInfo Structure"))
  (return (`self.Resources`)))

(fn `SetCharacterAvatar`
  (if (> (`KismetArrayLibrary.Array_Length` (`self.AvatarsInfo`)) 0)
    (for (_array_element _array_index) (`self.AvatarsInfo`)
      (switch `string` (`KismetTextLibrary.Conv_TextToString` (`.Genre_11_578941E1422EFBF96DFCCAA934930F6E` (break `/Game/Blueprints/Data/CharacterInfo` _array_element)))
        (:`F`
          (bind _structout (setmembers `/Game/Blueprints/Data/CharacterInfo` :`StructRef` _array_element :`Thumbnail` (make `SlateBrush` (32.0 32.0) (struct) (struct :`SpecifiedColor` (struct :`R` 1.0 :`G` 1.0 :`B` 1.0 :`A` 1.0) :`ColorUseRule` "UseColor_Specified") (`|GetArrayItem` (`self.AvatarsFemales`) (`KismetMathLibrary.RandomIntegerInRange` 0 (- (`KismetArrayLibrary.Array_Length` (`self.AvatarsFemales`)) 1))))))
          (`KismetArrayLibrary.Array_Set` (`self.AvatarsInfo`) _array_index _structout))
        (:`M`
          (bind _structout_2 (setmembers `/Game/Blueprints/Data/CharacterInfo` :`StructRef` _array_element :`Thumbnail` (make `SlateBrush` (32.0 32.0) (struct) (struct :`SpecifiedColor` (struct :`R` 1.0 :`G` 1.0 :`B` 1.0 :`A` 1.0) :`ColorUseRule` "UseColor_Specified") (`|GetArrayItem` (`self.AvatarsMales`) (`KismetMathLibrary.RandomIntegerInRange` 0 (- (`KismetArrayLibrary.Array_Length` (`self.AvatarsMales`)) 1))))))
          (`KismetArrayLibrary.Array_Set` (`self.AvatarsInfo`) _array_index _structout_2))))))

(fn `SetCharacterInfo`
  (bind _outrownames (`DataTableFunctionLibrary.GetDataTableRowNames` "/Game/Blueprints/Data/DT_CharaterInfo.DT_CharaterInfo"))
  (for _array_element _outrownames
    (bind _returnvalue (`|GetDataTableRow` "/Game/Blueprints/Data/DT_CharaterInfo.DT_CharaterInfo" _array_element)
      (:`then`
        (`KismetArrayLibrary.Array_Add` (`self.AvatarsInfo`) _returnvalue))))
  (`self.SetCharacterAvatar`))

(fn `UserConstructionScript`)