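; BP_Campfire is a selectable campfire that shows an info widget while selected.
; It extends its parent's selection events: OnSelect creates and stores a WBP_CampfireInfo widget and adds it to the viewport, and OnDeselect removes it.
; Input-mode switching nodes are present but unconnected, and construction only calls the parent.
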(event `self.OnSelect`
  (`parent.OnSelect`)
  (bind _returnvalue (`|CreateWidget` "/Game/Widget/WBP_CampfireInfo.WBP_CampfireInfo_C" (`GameplayStatics.GetPlayerController` 0)))
  (`UserWidget.AddToViewport` _returnvalue 0)
  (bind _output_get (set `self.Widget` _returnvalue)))

(event `self.OnDeselect`
  (`parent.OnDeselect`)
  (`Widget.RemoveFromParent` (`self.Widget`)))

(fn `UserConstructionScript`
  (`parent.UserConstructionScript`))